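; First-person player character Blueprint that handles movement, look, jump and sprint input.
; Axis events feed pitch and yaw to the controller and apply movement along the actor's forward and right vectors, with separate back and left axes using those same vectors unnegated.
; Sprint switches the CharacterMovement max walk speed on press and release, while Jump uses the built-in Character jump functions.
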(event EventBeginPlay)

(event Collision|EventActorBeginOverlap
  (params (OtherActor :type Actor%20Object%20Reference)))

(event EventTick
  (params (DeltaSeconds :type Float%20%28single-precision%29)))

(event Input|ActionEvents|InputActionJump
  (params (Key :type Key%20Structure :default "None"))
  ;[0.03205 0.15 0.03621 0.5] Movement
  (:Pressed
    (Character|Jump))
  (:Released
    (Character|StopJumping)))

(event Input|ActionEvents|InputActionSprint
  (params (Key :type Key%20Structure :default "None"))
  (bind _charactermovement (Variables|Character|GetCharacterMovement))
  ;[0.03205 0.15 0.03621 0.5] Movement
  (:Pressed
    (Variables|/Script/Engine.CharacterMovementComponent|SetMaxWalkSpeed _charactermovement 6e+02))
  (:Released
    (Variables|/Script/Engine.CharacterMovementComponent|SetMaxWalkSpeed _charactermovement 4e+02)))

(event Input|AxisEvents|InputAxisMoveForward
  (params (AxisValue :type Float%20%28single-precision%29))
  ;[0.03205 0.15 0.03621 0.5] Movement
  (Pawn|Input|AddMovementInput (Transformation|GetActorForwardVector) AxisValue false))

(event Input|AxisEvents|InputAxisMoveBack
  (params (AxisValue :type Float%20%28single-precision%29))
  ;[0.03205 0.15 0.03621 0.5] Movement
  (Pawn|Input|AddMovementInput (Transformation|GetActorForwardVector) AxisValue false))

(event Input|AxisEvents|InputAxisMoveRight
  (params (AxisValue :type Float%20%28single-precision%29))
  ;[0.03205 0.15 0.03621 0.5] Movement
  (Pawn|Input|AddMovementInput (Transformation|GetActorRightVector) AxisValue false))

(event Input|AxisEvents|InputAxisMoveLeft
  (params (AxisValue :type Float%20%28single-precision%29))
  ;[0.03205 0.15 0.03621 0.5] Movement
  (Pawn|Input|AddMovementInput (Transformation|GetActorRightVector) AxisValue false))

(event Input|AxisEvents|InputAxisLookPitch
  (params (AxisValue :type Float%20%28single-precision%29))
  ;[0.03205 0.15 0.03621 0.5] Movement
  (Pawn|Input|AddControllerPitchInput AxisValue))

(event Input|AxisEvents|InputAxisLookYaw
  (params (AxisValue :type Float%20%28single-precision%29))
  ;[0.03205 0.15 0.03621 0.5] Movement
  (Pawn|Input|AddControllerYawInput AxisValue))

(fn ConstructionScript)